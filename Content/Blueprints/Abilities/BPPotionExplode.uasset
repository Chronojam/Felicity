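; Potion actor that explodes on contact or on a timed fuse.
; It arms shortly after spawning, then detonates when its box overlaps anything other than a ThrowablePotion or when the fuse runs out.
; A guarded one-shot detonation fires a radial impulse, plays upright particles and a sound, and hides the mesh and stops its physics.
; The actor destroys itself when the particle system finishes.
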(event OnComponentBeginOverlap(Box)
  (params (OverlappedComponent :type Primitive%20Component%20Object%20Reference) (OtherActor :type Actor%20Object%20Reference) (OtherComp :type Primitive%20Component%20Object%20Reference) (OtherBodyIndex :type Integer) (bFromSweep :type Boolean) (SweepResult :type Hit%20Result%20Structure%20%28by%20ref%29))
  (bind _particlesystem (Variables|Default|GetParticleSystem))
  (bind _staticmesh (Variables|Default|GetStaticMesh))
  (Utilities|Casting|CastToThrowablePotion OtherActor
    (:CastFailed
      (if (and (Variables|Default|GetCanExplode) (not (Variables|Default|GetExploding)))
        (Variables|Default|SetExploding true)
        (Utilities|FlowControl|Sequence
          (:then_0
            (Class|RadialForceComponent|FireImpulse (Variables|Default|GetRadialForce)))
          (:then_1
            (Transformation|SetWorldRotation _particlesystem "0, 0, 0" false false))
          (:then_2
            (Components|Activation|Activate _particlesystem false)
            (Audio|PlaySoundatLocation 0 (Transformation|GetActorLocation) "0, 0, 0" 1.0 1.0 0.0 0 0 0)
            (Rendering|SetVisibility _staticmesh false false)
            (Physics|SetSimulatePhysics _staticmesh false)))))))

(event OnSystemFinished(ParticleSystem)
  (params (PSystem :type Particle%20System%20Component%20Object%20Reference))
  (Actor|DestroyActor))

(event EventBeginPlay
  (bind _particlesystem (Variables|Default|GetParticleSystem))
  (bind _staticmesh (Variables|Default|GetStaticMesh))
  (Utilities|FlowControl|Delay 0.3)
  (Variables|Default|SetCanExplode true)
  (Utilities|FlowControl|Delay 5.0)
  (if (and (Variables|Default|GetCanExplode) (not (Variables|Default|GetExploding)))
    (Variables|Default|SetExploding true)
    (Utilities|FlowControl|Sequence
      (:then_0
        (Class|RadialForceComponent|FireImpulse (Variables|Default|GetRadialForce)))
      (:then_1
        (Transformation|SetWorldRotation _particlesystem "0, 0, 0" false false))
      (:then_2
        (Components|Activation|Activate _particlesystem false)
        (Audio|PlaySoundatLocation 0 (Transformation|GetActorLocation) "0, 0, 0" 1.0 1.0 0.0 0 0 0)
        (Rendering|SetVisibility _staticmesh false false)
        (Physics|SetSimulatePhysics _staticmesh false)))))

(event Collision|EventActorBeginOverlap
  (params (OtherActor :type Actor%20Object%20Reference)))

(event EventTick
  (params (DeltaSeconds :type Float%20%28single-precision%29)))

(fn ConstructionScript)