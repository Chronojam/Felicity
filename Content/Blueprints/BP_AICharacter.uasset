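; BP_AICharacter is an AI character that walks an endless patrol route between four waypoint actors.
; BeginPlay lowers the walk speed and calls the Patrol event, which chains AI MoveTo nodes through Waypoint01 to Waypoint04 with a short delay after each arrival.
; After the last waypoint Patrol calls itself to loop, while any failed move prints that waypoint's label and ends the patrol.
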(event Custom|Patrol
  (AI|AIMoveTo self "0, 0, 0" (Variables|Default|GetWaypoint%2001) 5.0 false
    (:OnSuccess
      (Utilities|FlowControl|Delay 0.2)
      (AI|AIMoveTo self "0, 0, 0" (Variables|Default|GetWaypoint%2002) 5.0 false
        (:OnSuccess
          (Utilities|FlowControl|Delay 0.2)
          (AI|AIMoveTo self "0, 0, 0" (Variables|Default|GetWaypoint%2003) 5.0 false
            (:OnSuccess
              (Utilities|FlowControl|Delay 0.2)
              (AI|AIMoveTo self "0, 0, 0" (Variables|Default|GetWaypoint%2004) 5.0 false
                (:OnSuccess
                  (Utilities|FlowControl|Delay 0.2)
                  (CallFunction|Patrol))
                (:OnFail
                  (Development|PrintString "W4"))))
            (:OnFail
              (Development|PrintString "W3"))))
        (:OnFail
          (Development|PrintString "W2"))))
    (:OnFail
      (Development|PrintString "W1"))))

(event EventBeginPlay
  (Variables|/Script/Engine.CharacterMovementComponent|SetMaxWalkSpeed (Variables|Character|GetCharacterMovement) 2e+02)
  (CallFunction|Patrol))

(event Collision|EventActorBeginOverlap
  (params (OtherActor :type Actor%20Object%20Reference)))

(event EventTick
  (params (DeltaSeconds :type Float%20%28single-precision%29)))

(fn ConstructionScript)